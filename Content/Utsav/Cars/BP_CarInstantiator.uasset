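; BP_CarInstantiator is a traffic spawner that endlessly spawns BP_Car1 cars at its root and also destroys cars entering its BoxCollider.
; On BeginPlay its own yaw sets DrivingLeft, true only at exactly zero, which picks each car's facing and is copied onto the car.
; InstantiateCars calls itself after a short random delay to keep the stream going.
; BoxCollider overlaps destroy any BP_Car1 or subclass and print a debug message.
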(event OnComponentBeginOverlap(BoxCollider)
  (params (OverlappedComponent :type Primitive%20Component%20Object%20Reference) (OtherActor :type Actor%20Object%20Reference) (OtherComp :type Primitive%20Component%20Object%20Reference) (OtherBodyIndex :type Integer) (bFromSweep :type Boolean) (SweepResult :type Hit%20Result%20Structure%20%28by%20ref%29))
  ;[1 1 1] Destroy Cars
  (if (Utilities|ClassIsChildOf (Utilities|GetClass OtherActor) "/Game/Utsav/Cars/BP_Car1.BP_Car1_C")
    (Actor|DestroyActor OtherActor)
    (Development|PrintString "DESTROY")))

(event Custom|InstantiateCars
  (bind _returnvalue (Game|SpawnActorfromClass "/Game/Utsav/Cars/BP_Car1.BP_Car1_C" (Math|Transform|MakeTransform (Transformation|GetWorldLocation (Variables|Default|GetDefaultSceneRoot self)) (Math|Rotator|MakeRotator 0.0 0.0 (Math|Float|SelectFloat 0.0 1.8e+02 (Variables|Default|GetDrivingLeft?))) "1.000000,1.000000,1.000000") "Undefined" 0 0))
  (bind _asbp_car_1 (Utilities|Casting|CastToBP_Car1 _returnvalue))
  (Variables|/Game/Utsav/Cars/BP_Car1.BP_Car1_C|SetDrivingLeft _asbp_car_1 (Variables|Default|GetDrivingLeft?))
  (Utilities|FlowControl|Delay (Math|Random|RandomFloatinRange 1.5 3.0))
  (CallFunction|InstantiateCars))

(event EventBeginPlay
  (Math|Float|CompareFloat (.yaw (Transformation|GetActorRotation self)) 0.0
    (:>
      (Variables|Default|SetDrivingLeft? false :!label _label))
    (:==
      (Variables|Default|SetDrivingLeft? true))
    (:<
      (goto _label)))
  (CallFunction|InstantiateCars))

(event Collision|EventActorBeginOverlap
  (params (OtherActor :type Actor%20Object%20Reference)))

(event EventTick
  (params (DeltaSeconds :type Float%20%28single-precision%29)))

(fn ConstructionScript)