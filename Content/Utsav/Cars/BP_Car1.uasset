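; BP_Car1 is a car actor that drives endlessly along the world X axis with a randomly chosen look and speed.
; On BeginPlay it picks a skeletal mesh from CarTypes, rolls CarSpeed and starts CarMove.
; CarMove uses MoveComponentTo to shift the capsule by CarSpeed, with DrivingLeft selecting direction and yaw, then calls itself again to keep the car moving without Tick.
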(event Custom|CarMove
  (bind _self self)
  (bind _carspeed (Variables|Default|GetCarSpeed))
  (bind _drivingleft (Variables|Default|GetDrivingLeft))
  (bind _returnvalue (Transformation|GetActorLocation _self))
  (bind _returnvalue_2 (Math|Float|MakeLiteralFloat _carspeed))
  ;[1 1 1] Car Moving Code
  (Components|MoveComponentTo (Variables|Collision|GetCapsuleComponent) (Math|Vector|MakeVector (+ (.x _returnvalue) (Math|Float|SelectFloat _returnvalue_2 (* _returnvalue_2 -1.0) _drivingleft)) (.y _returnvalue) (.z _returnvalue)) (Math|Rotator|MakeRotator 0.0 0.0 (Math|Float|SelectFloat 0.0 1.8e+02 _drivingleft)) false false 0.2 false)
  (CallFunction|CarMove))

(event EventBeginPlay
  (Components|SkeletalMesh|SetSkeletalMeshAsset (Variables|Character|GetMesh) (.OutItem (Utilities|Array|Random (Variables|Default|GetCarTypes))))
  (Variables|Default|SetCarSpeed (Math|Random|RandomFloatinRange 175.0 2e+02))
  (CallFunction|CarMove))

(event Collision|EventActorBeginOverlap
  (params (OtherActor :type Actor%20Object%20Reference)))

(event EventTick
  (params (DeltaSeconds :type Float%20%28single-precision%29)))

(fn ConstructionScript)