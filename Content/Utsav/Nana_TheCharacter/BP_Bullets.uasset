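; Bullet actor whose sphere collider kills BP_AI enemies with a slipping death when it overlaps one of their box components.
; The overlap flags DidSlip on the enemy's anim blueprint, zeroes its walk speed and disables its Box collision.
; It then calls DeathCounter on a BP_KeyManager found in the level and destroys the enemy after a short delay.
; The StopActiveMovement and blackboard isDead nodes are unconnected.
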(event OnComponentBeginOverlap(SphereCollider)
  (params (OverlappedComponent :type Primitive%20Component%20Object%20Reference) (OtherActor :type Actor%20Object%20Reference) (OtherComp :type Primitive%20Component%20Object%20Reference) (OtherBodyIndex :type Integer) (bFromSweep :type Boolean) (SweepResult :type Hit%20Result%20Structure%20%28by%20ref%29))
  ;[1 1 1] Slipping Code
  (if (and (Utilities|ClassIsChildOf (Utilities|GetClass OtherComp) "/Script/Engine.BoxComponent") (Utilities|ClassIsChildOf (Utilities|GetClass OtherActor) "/Game/Utsav/Enemies/EnemyAI/BP_AI.BP_AI_C"))
    (bind _asbp_ai (Utilities|Casting|CastToBP_AI OtherActor))
    (bind _asabp_enemy_ai (Utilities|Casting|CastToABP_EnemyAI (Components|SkeletalMesh|GetAnimInstance (Variables|/Script/Engine.Character|GetMesh _asbp_ai))))
    (Variables|/Game/Utsav/Enemies/Animations/ABP_EnemyAI.ABP_EnemyAI_C|SetdidSlip? _asabp_enemy_ai true)
    (Variables|/Script/Engine.CharacterMovementComponent|SetMaxWalkSpeed (Variables|/Script/Engine.Character|GetCharacterMovement _asbp_ai) (Math|Float|MakeLiteralFloat 0.0))
    (Collision|SetCollisionEnabled (Variables|/Game/Utsav/Enemies/EnemyAI/BP_AI.BP_AI_C|GetBox _asbp_ai) "NoCollision")
    (bind _outactors (Actor|GetAllActorsOfClass "/Game/Utsav/Key/BP_KeyManager.BP_KeyManager_C"))
    (Default|DeathCounter (.OutItem (Utilities|Array|Random _outactors)))
    (Development|PrintString "DEATH")
    (Utilities|FlowControl|Delay 0.6)
    (Actor|DestroyActor OtherActor)))

(event EventBeginPlay)

(event Collision|EventActorBeginOverlap
  (params (OtherActor :type Actor%20Object%20Reference)))

(event EventTick
  (params (DeltaSeconds :type Float%20%28single-precision%29)))

(fn ConstructionScript)