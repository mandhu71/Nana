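; Enemy AI character that wanders, chases the player to attack, and slips and dies when shot.
; RandomWalk and FollowPlayer loop through AI MoveTo success, with chasing triggered by PawnSensing while the box collision flags the player in range.
; Reaching the player briefly pulses InRange on ABP_EnemyAI for a stomp.
; A BP_Bullets overlap on the sphere sets DidSlip, clears IsAlive and stops movement.
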(event OnSeePawn(PawnSensing)
  (params (Pawn :type Pawn%20Object%20Reference))
  (if (Variables|Default|GetisPlayerInRange?)
    (Variables|Default|SetisSeeingPlayer? true)
    (CallFunction|FollowPlayer)))

(event OnComponentBeginOverlap(SphereCollision)
  (params (OverlappedComponent :type Primitive%20Component%20Object%20Reference) (OtherActor :type Actor%20Object%20Reference) (OtherComp :type Primitive%20Component%20Object%20Reference) (OtherBodyIndex :type Integer) (bFromSweep :type Boolean) (SweepResult :type Hit%20Result%20Structure%20%28by%20ref%29))
  ;[1 1 1] Slipping Code
  (if (Utilities|ClassIsChildOf (Utilities|GetClass OtherActor) "/Game/Utsav/Nana_TheCharacter/BP_Bullets.BP_Bullets_C")
    (bind _asabp_enemy_ai (Utilities|Casting|CastToABP_EnemyAI (Components|SkeletalMesh|GetAnimInstance (Variables|Character|GetMesh))))
    (Variables|/Game/Utsav/Enemies/Animations/ABP_EnemyAI.ABP_EnemyAI_C|SetdidSlip? _asabp_enemy_ai true)
    (Utilities|FlowControl|Delay 0.2)
    (Variables|Default|SetisAlive? false)
    (CallFunction|Dead)))

(event OnComponentBeginOverlap(BoxCollision)
  (params (OverlappedComponent :type Primitive%20Component%20Object%20Reference) (OtherActor :type Actor%20Object%20Reference) (OtherComp :type Primitive%20Component%20Object%20Reference) (OtherBodyIndex :type Integer) (bFromSweep :type Boolean) (SweepResult :type Hit%20Result%20Structure%20%28by%20ref%29))
  ;[1 1 1] Capsule Collider Logic
  (if (Collision|IsOverlappingActor OverlappedComponent (Game|GetPlayerCharacter 0) :!class /Script/Engine.PrimitiveComponent)
    (Development|PrintString "I SEE YOU")
    (Variables|Default|SetisPlayerInRange? true)))

(event OnComponentEndOverlap(BoxCollision)
  (params (OverlappedComponent :type Primitive%20Component%20Object%20Reference) (OtherActor :type Actor%20Object%20Reference) (OtherComp :type Primitive%20Component%20Object%20Reference) (OtherBodyIndex :type Integer))
  ;[1 1 1] Capsule Collider Logic
  (Variables|Default|SetisPlayerInRange? false)
  (CallFunction|RandomWalk))

(event Custom|Dead
  ;[1 1 1] Stop Moving
  (Class|NavMovementComponent|StopActiveMovement (Variables|Character|GetCharacterMovement)))

(event Custom|RandomWalk
  ;[1 1 1] Random Walk Enemy
  (if (Variables|Default|GetisAlive?)
    (Variables|/Script/Engine.CharacterMovementComponent|SetMaxWalkSpeed (Variables|Character|GetCharacterMovement self) (Math|Float|MakeLiteralFloat 1e+02))
    (AI|AIMoveTo self (.RandomLocation (AI|Navigation|GetRandomReachablePointinRadius (Transformation|GetActorLocation) 2.5e+03 0 0)) 0 5.0 false
      (:OnSuccess
        (CallFunction|RandomWalk)))))

(event Custom|FollowPlayer
  (bind _mesh (Variables|Character|GetMesh))
  (bind _returnvalue (Components|SkeletalMesh|GetAnimInstance _mesh))
  ;[1 1 1] Follow Player Enemy
  (if (Variables|Default|GetisAlive?)
    (Variables|Default|SetcanAttack? (Variables|Default|GetisSeeingPlayer?))
    (if (Variables|Default|GetisSeeingPlayer?)
      (Variables|/Script/Engine.CharacterMovementComponent|SetMaxWalkSpeed (Variables|Character|GetCharacterMovement self) (Math|Float|MakeLiteralFloat 2e+02))
      (AI|AIMoveTo self (Transformation|GetActorLocation (Game|GetPlayerCharacter 0)) 0 7e+01 false
        (:OnSuccess
          (bind _asabp_enemy_ai (Utilities|Casting|CastToABP_EnemyAI _returnvalue))
          (Variables|/Game/Utsav/Enemies/Animations/ABP_EnemyAI.ABP_EnemyAI_C|SetinRange? _asabp_enemy_ai true)
          (Development|PrintString "STOMP")
          (Utilities|FlowControl|Delay 0.2)
          (bind _asabp_enemy_ai_2 (Utilities|Casting|CastToABP_EnemyAI _returnvalue))
          (Variables|/Game/Utsav/Enemies/Animations/ABP_EnemyAI.ABP_EnemyAI_C|SetinRange? _asabp_enemy_ai_2 false)
          (if (Variables|Default|GetisPlayerInRange?)
            (CallFunction|FollowPlayer)
            (else
              (Variables|Default|SetisSeeingPlayer? false)
              (CallFunction|RandomWalk)))))
      (else
        (CallFunction|RandomWalk)))))

(event EventBeginPlay
  (Variables|Default|SetisPlayerInRange? false)
  (CallFunction|RandomWalk))

(event Collision|EventActorBeginOverlap
  (params (OtherActor :type Actor%20Object%20Reference)))

(event EventTick
  (params (DeltaSeconds :type Float%20%28single-precision%29)))

(fn ConstructionScript)